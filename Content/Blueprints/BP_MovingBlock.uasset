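; Moving block that slides its Cube between a start and end location depending on the inherited lock state.
; Each Tick, LiftUp or LiftDown advances or rewinds a Timer bounded by Duration, whose ratio lerps the relative location, so movement reverses smoothly mid-travel.
; Lock and Unlock only forward to the parent.
; A Lift timeline version of the same motion remains in the graph but never runs.
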(event EventLock
  (|CallParentFunction))

(event EventUnlock
  (|CallParentFunction))

(event EventBeginPlay
  (|CallParentFunction)
  (Variables|Default|SetTimer 0.0))

(event EventTick
  (params (DeltaSeconds :type Float%20%28single-precision%29))
  (if (Variables|Default|GetbIsUnlocked)
    (CallFunction|LiftUp DeltaSeconds)
    (else
      (CallFunction|LiftDown DeltaSeconds))))

(fn ConstructionScript)

(fn LiftUp
  (params (DeltaTime :type Float%20%28double-precision%29))
  (if (< (Variables|Default|GetTimer) (Variables|Config|GetDuration))
    (Variables|Default|SetTimer (+ DeltaTime (Variables|Default|GetTimer)))
    (Transformation|SetRelativeLocation (Variables|Default|GetCube) (Math|Vector|Lerp(Vector) (Variables|Config|GetStartLocation) (Variables|Config|GetEndLocation) (Math|Float|Clamp(Float) (/ (Variables|Default|GetTimer) (Variables|Config|GetDuration)))) false false)
    (else
      (Variables|Default|SetTimer (Variables|Config|GetDuration)))))

(fn LiftDown
  (params (DeltaTime :type Float%20%28double-precision%29))
  (if (> (Variables|Default|GetTimer) 0.0)
    (Variables|Default|SetTimer (- (Variables|Default|GetTimer) DeltaTime))
    (Transformation|SetRelativeLocation (Variables|Default|GetCube) (Math|Vector|Lerp(Vector) (Variables|Config|GetStartLocation) (Variables|Config|GetEndLocation) (Math|Float|Clamp(Float) (/ (Variables|Default|GetTimer) (Variables|Config|GetDuration)))) false false)
    (else
      (Variables|Default|SetTimer 0.0))))