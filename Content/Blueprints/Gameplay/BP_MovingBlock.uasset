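; Moving block that slides its Cube between StartLocation and EndLocation in response to lock state changes.
; OnLockChangedState plays the Lift timeline forward on unlock and reverses it on lock, with play rate set to 1/Duration.
; The timeline alpha lerps the Cube's relative location.
; Timer-based LiftUp and LiftDown functions offer the same motion, but their only calls sit in unreachable graph code and Tick is empty.
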(event EventOnLockChangedState
  (params (bIsUnlocked :type Boolean))
  (if bIsUnlocked
    (Components|Timeline|SetPlayRate (Variables|Default|GetLift) (/ 1.0 (Variables|Config|GetDuration)))
    (bind _lift (Timeline|Lift Play)
      (:Update
        (Transformation|SetRelativeLocation (Variables|Default|GetCube) (Math|Vector|Lerp(Vector) (Variables|Config|GetStartLocation) (Variables|Config|GetEndLocation) _lift) false false)))
    (else
      (Components|Timeline|SetPlayRate (Variables|Default|GetLift) (/ 1.0 (Variables|Config|GetDuration)))
      (Timeline|Lift Reverse))))

(event EventBeginPlay
  (|CallParentFunction)
  (Variables|Default|SetTimer 0.0))

(event EventTick
  (params (DeltaSeconds :type Float%20%28single-precision%29)))

(fn ConstructionScript)

(fn LiftUp
  (params (DeltaTime :type Float%20%28double-precision%29))
  (if (< (Variables|Default|GetTimer) (Variables|Config|GetDuration))
    (Variables|Default|SetTimer (+ DeltaTime (Variables|Default|GetTimer)))
    (Transformation|SetRelativeLocation (Variables|Default|GetCube) (Math|Vector|Lerp(Vector) (Variables|Config|GetStartLocation) (Variables|Config|GetEndLocation) (Math|Float|Clamp(Float) (/ (Variables|Default|GetTimer) (Variables|Config|GetDuration)))) false false)
    (else
      (Variables|Default|SetTimer (Variables|Config|GetDuration)))))

(fn LiftDown
  (params (DeltaTime :type Float%20%28double-precision%29))
  (if (> (Variables|Default|GetTimer) 0.0)
    (Variables|Default|SetTimer (- (Variables|Default|GetTimer) DeltaTime))
    (Transformation|SetRelativeLocation (Variables|Default|GetCube) (Math|Vector|Lerp(Vector) (Variables|Config|GetStartLocation) (Variables|Config|GetEndLocation) (Math|Float|Clamp(Float) (/ (Variables|Default|GetTimer) (Variables|Config|GetDuration)))) false false)
    (else
      (Variables|Default|SetTimer 0.0))))