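; BP_Trigger is a trigger volume that unlocks and locks a key as actors enter and leave it.
; It counts overlapping actors, calling ServerUnlockKey on every entry and ServerLockKey when the count drops to zero or below, then clamping it to zero.
; Before either call, it sets the overlapping actor as its owner.
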(event OnComponentBeginOverlap(TriggerBox)
  (params (OverlappedComponent :type Primitive%20Component%20Object%20Reference) (OtherActor :type Actor%20Object%20Reference) (OtherComp :type Primitive%20Component%20Object%20Reference) (OtherBodyIndex :type Integer) (bFromSweep :type Boolean) (SweepResult :type Hit%20Result%20Structure%20%28by%20ref%29))
  (Math|Integer|IncrementInt (Variables|Default|GetPeopleInsideTrigger)
    (:%20%20
      (Actor|SetOwner OtherActor)
      (Class|KeyActor|ServerUnlockKey))))

(event OnComponentEndOverlap(TriggerBox)
  (params (OverlappedComponent :type Primitive%20Component%20Object%20Reference) (OtherActor :type Actor%20Object%20Reference) (OtherComp :type Primitive%20Component%20Object%20Reference) (OtherBodyIndex :type Integer))
  (Math|Integer|DecrementInt (Variables|Default|GetPeopleInsideTrigger)
    (:%20%20
      (if (<= (Variables|Default|GetPeopleInsideTrigger) 0)
        (Actor|SetOwner OtherActor)
        (Class|KeyActor|ServerLockKey)
        (Variables|Default|SetPeopleInsideTrigger 0)))))

(fn ConstructionScript)